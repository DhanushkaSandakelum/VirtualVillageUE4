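; BP_Nav_Waypoint is an NPC system navigation waypoint marker that carries a group name and an ID.
; The construction script writes both to text components and applies visibility settings to the group label and its children and to the sphere marker, including whether the sphere hides in game.
; Fn_SetWaypointInfo refreshes both labels on demand; the actor runs no event logic of its own.
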(fn `Fn_SetWaypointInfo`
  (`TextRenderComponent.K2_SetText` (`self.PathName`) (`self.WaypointGroupName`))
  (`TextRenderComponent.K2_SetText` (`self.ID`) (`KismetTextLibrary.Conv_IntToText` (`self.WaypointID`))))

(fn `UserConstructionScript`
  (`TextRenderComponent.K2_SetText` (`self.PathName`) (`self.WaypointGroupName`))
  (`TextRenderComponent.K2_SetText` (`self.ID`) (`KismetTextLibrary.Conv_IntToText` (`self.WaypointID`)))
  ;[0 0 0] Visibilities
  (`SceneComponent.SetVisibility` (`self.PathName`) (`self.TextVisible?`) true)
  (`SceneComponent.SetVisibility` (`self.Sphere`) (`self.MarkerVisible?`) false)
  (`SceneComponent.SetHiddenInGame` (`self.Sphere`) (`self.MarkerHidden?`) false))