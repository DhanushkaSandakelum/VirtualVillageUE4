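; BP_Nav_Path is a spline-based NPC navigation path that generates BP_Nav_Waypoint actors along its points.
; The construction script applies looping and visibility settings to the spline.
; Placing waypoints optionally destroys those tagged with the PathID, then traces down from each spline point and spawns a waypoint at a floor offset.
; Each waypoint receives the PathID as tag and group plus its point index, and a separate event deletes them by tag.
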(event `Ev_DestroyCurrentWaypoints`
  (bind _outactors (`GameplayStatics.GetAllActorsWithTag` (`self.WaypointTag`)))
  (for _array_element _outactors
    (`self.K2_DestroyActor` _array_element))
  (`self.Ev_SpawnWaypoints`))

(event `Ev_SpawnWaypoints`
  (bind _returnvalue (`SplineComponent.GetLocationAtSplinePoint` (`self.Spline`) (`self.CurrentIndex`) "World"))
  (`KismetArrayLibrary.Array_Clear` (`self.ListOfWaypoints`))
  (for _index (range (`SplineComponent.GetNumberOfSplinePoints` (`self.Spline`)))
    (set `self.CurrentIndex` _index)
    (bind _outhit (`KismetSystemLibrary.LineTraceSingle` _returnvalue (+ _returnvalue (* (* (`KismetMathLibrary.GetUpVector` (`SceneComponent.K2_GetComponentRotation` (`self.DefaultSceneRoot`))) -1.0) (`self.TraceDistance`))) "TraceTypeQuery1"))
    (bind _returnvalue_2 (`|SpawnActorFromClass` "/Game/VV/SubSystems/NPCSystemV5/Blueprints/Navigations/BP_Nav_Waypoint.BP_Nav_Waypoint_C" (`KismetMathLibrary.MakeTransform` (+ (`.Location` (`GameplayStatics.BreakHitResult` _outhit)) (`KismetMathLibrary.MakeVector` 0.0 0.0 (`self.FloorOffset`)))) "Undefined" "OverrideRootScale" null null))
    (set `self.WaypointRef` _returnvalue_2)
    (`KismetArrayLibrary.Array_Add` (`self.ListOfWaypoints`) (`self.WaypointRef`))
    (`KismetArrayLibrary.Array_Clear` (`self.Tag`))
    (`KismetArrayLibrary.Array_Add` (`self.Tag`) (`KismetStringLibrary.Conv_StringToName` (`KismetTextLibrary.Conv_TextToString` (`self.PathID`))))
    (set `Actor.Tags` (`self.Tag`) (`self.WaypointRef`))
    (set `/Game/VV/SubSystems/NPCSystemV5/Blueprints/Navigations/BP_Nav_Waypoint.WaypointGroupName` (`self.PathID`) (`self.WaypointRef`))
    (set `/Game/VV/SubSystems/NPCSystemV5/Blueprints/Navigations/BP_Nav_Waypoint.WaypointID` (`self.CurrentIndex`) (`self.WaypointRef`))
    (`/Game/VV/SubSystems/NPCSystemV5/Blueprints/Navigations/BP_Nav_Waypoint.Fn_SetWaypointInfo` (`self.WaypointRef`))))

(event `1_PlaceWaypoints`
  (if (`self.DestroyOldWaypoints?`)
    (set `self.WaypointTag` (`KismetStringLibrary.Conv_StringToName` (`KismetTextLibrary.Conv_TextToString` (`self.PathID`))))
    (`self.Ev_DestroyCurrentWaypoints`)
    (else
      (`self.Ev_SpawnWaypoints`))))

(event `2_DeleteWaypoints`
  (set `self.WaypointTag` (`KismetStringLibrary.Conv_StringToName` (`KismetTextLibrary.Conv_TextToString` (`self.PathID`))))
  (bind _outactors (`GameplayStatics.GetAllActorsWithTag` (`self.WaypointTag`)))
  (for _array_element _outactors
    (`self.K2_DestroyActor` _array_element)))

(fn `UserConstructionScript`
  (`SplineComponent.SetClosedLoop` (`self.Spline`) (`self.IsPathLooped?`) true)
  ;[0 0 0] Visibilities
  (`SceneComponent.SetVisibility` (`self.Spline`) (`self.ShowSpline?`) false)
  (`SceneComponent.SetHiddenInGame` (`self.Spline`) (`self.HideSpline?`) false))