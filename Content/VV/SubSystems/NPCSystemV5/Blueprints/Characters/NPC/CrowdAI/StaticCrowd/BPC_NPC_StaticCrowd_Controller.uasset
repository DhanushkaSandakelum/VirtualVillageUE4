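; Actor component that drives static crowd NPC Characters through randomly chosen montage animations with optional sound.
; When active, it forces a mesh LOD on BeginPlay, calls an empty optimization stub, then waits up to a second at random.
; Each cycle picks an animation entry, chains start, cycle and stop montages on blend-out, skipping missing clips, then repeats with a new pick.
; The entry's sound plays at the owner's location alongside the cycle montage.
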(event `self.ReceiveBeginPlay`
  (bind _ascharacter (cast `Character` (`self.GetOwner`)))
  (set `self.Owner` _ascharacter)
  (if (`self.Active?`)
    (`SkinnedMeshComponent.SetForcedLOD` (`Character.Mesh` (`self.Owner`)) (`self.MeshForcedLOD`))
    (`self.Fn_OptimizeNPC`)
    (`KismetSystemLibrary.Delay` (`KismetMathLibrary.RandomFloatInRange` 0.0 1.0))
    (`self.Ev_PlayIntroAnim`)))

(event `Ev_PlayIntroAnim`
  (bind _animationlist (`self.AnimationList`))
  (if (`KismetArrayLibrary.Array_IsValidIndex` (`self.AnimationList`))
    (set `self.SelectedAnimation` (`|GetArrayItem` _animationlist (`KismetMathLibrary.RandomIntegerInRange` 0 (`KismetArrayLibrary.Array_LastIndex` _animationlist))))
    (`/Engine/EditorBlueprintResources/StandardMacros.IsValid` (`.StartClip_3_8103E6A3466B58AA2D55449EA865C04F` (break `/Game/VV/SubSystems/NPCSystemV5/Data/Structs/S_NPC_Animation` (`self.SelectedAnimation`)))
      (:`Is Valid`
        (`|PlayMontage` (`Actor.GetComponentByClass` (`self.Owner`) "/Script/Engine.SkeletalMeshComponent") (`.StartClip_3_8103E6A3466B58AA2D55449EA865C04F` (break `/Game/VV/SubSystems/NPCSystemV5/Data/Structs/S_NPC_Animation` (`self.SelectedAnimation`)))
          (:`OnBlendOut`
            (`self.Ev_PlayLoopAnim`))))
      (:`Is Not Valid`
        (`self.Ev_PlayLoopAnim`)))))

(event `Ev_PlayLoopAnim`
  (`/Engine/EditorBlueprintResources/StandardMacros.IsValid` (`.CycleClip_6_3797BD4644D432D629E76DA14FA7BC0F` (break `/Game/VV/SubSystems/NPCSystemV5/Data/Structs/S_NPC_Animation` (`self.SelectedAnimation`)))
    (:`Is Valid`
      (`|ExecutionSequence`
        (:`then_0`
          (`|PlayMontage` (`Actor.GetComponentByClass` (`self.Owner`) "/Script/Engine.SkeletalMeshComponent") (`.CycleClip_6_3797BD4644D432D629E76DA14FA7BC0F` (break `/Game/VV/SubSystems/NPCSystemV5/Data/Structs/S_NPC_Animation` (`self.SelectedAnimation`)))
            (:`OnBlendOut`
              (`self.Ev_PlayOutroAnim`))))
        (:`then_1`
          (`self.Ev_PlaySound`))))
    (:`Is Not Valid`
      (`self.Ev_PlayOutroAnim`))))

(event `Ev_PlayOutroAnim`
  (`/Engine/EditorBlueprintResources/StandardMacros.IsValid` (`.StopClip_7_004F0C424AFC4B00E06782874AB26A98` (break `/Game/VV/SubSystems/NPCSystemV5/Data/Structs/S_NPC_Animation` (`self.SelectedAnimation`)))
    (:`Is Valid`
      (`|PlayMontage` (`Actor.GetComponentByClass` (`self.Owner`) "/Script/Engine.SkeletalMeshComponent") (`.StopClip_7_004F0C424AFC4B00E06782874AB26A98` (break `/Game/VV/SubSystems/NPCSystemV5/Data/Structs/S_NPC_Animation` (`self.SelectedAnimation`)))
        (:`OnBlendOut`
          (`self.Ev_PlayIntroAnim`))))
    (:`Is Not Valid`
      (`self.Ev_PlayIntroAnim`))))

(event `Ev_PlaySound`
  (bind (_sound_sound _sound_volume _sound_pitch _sound_starttime _sound_soundattenuation _sound_soundconcurrency) (break `/Game/VV/SubSystems/NPCSystemV5/Data/Structs/S_NPC_SoundInfo` (break `/Game/VV/SubSystems/NPCSystemV5/Data/Structs/S_NPC_Animation` (`self.SelectedAnimation`))))
  (bind (_returnvalue_location _returnvalue_rotation) (`KismetMathLibrary.BreakTransform` (`Actor.GetTransform` (`self.Owner`))))
  (`/Engine/EditorBlueprintResources/StandardMacros.IsValid` (`.Sound_12_FEC1C7D7445C5AB3D818309C2C93F315` (break `/Game/VV/SubSystems/NPCSystemV5/Data/Structs/S_NPC_SoundInfo` (`.Sound_10_C932628E4BC019B18CD1DBBF385F3914` (break `/Game/VV/SubSystems/NPCSystemV5/Data/Structs/S_NPC_Animation` (`self.SelectedAnimation`)))))
    (:`Is Valid`
      (`GameplayStatics.PlaySoundAtLocation` _sound_sound _returnvalue_location _returnvalue_rotation _sound_volume _sound_pitch _sound_starttime _sound_soundattenuation _sound_soundconcurrency null))))

(fn `Fn_OptimizeNPC`)