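; Base point-of-interest actor for the NPC system that spawns NPCs and assigns them stations.
; Editor events box-trace its area to collect stations, entrances and spawn points.
; The authority spawns listed NPCs in staggered batches at start or on player proximity, optionally despawning them and hiding station props.
; An occupancy map drives random, chance-based assignment of free, tag-matched stations, excluding unavailable ones, while NPCs can query their nearest entrance.
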(event `Ev_SpawnNPCs`
  (bind _spawnpoints (`self.SpawnPoints`))
  (bind _returnvalue (`self.GetComponentByClass` (`self.SpawnedNPC`) "/Game/VV/SubSystems/NPCSystemV5/Blueprints/Characters/NPC/GenericAI/BPC_NPCController.BPC_NPCController_C"))
  (bind (_npcclass _spawnamount) (break `/Game/VV/SubSystems/NPCSystemV5/Data/Structs/POI/S_POI_NPCs` (`|GetArrayItem` (`self.NPCList`) (`self.NPCIndex`))))
  (bind _area (`/Game/VV/SubSystems/NPCSystemV5/Blueprints/POIs/BaseClasses/BP_POI_NPCSpawner.Area` (`|GetArrayItem` _spawnpoints (`KismetMathLibrary.RandomIntegerInRange` 0 (`KismetArrayLibrary.Array_LastIndex` _spawnpoints)))))
  (`/Engine/EditorBlueprintResources/ActorMacros.Switch Has Authority`
    (:`Authority`
      (if (not (`self.NPCsSpawned`))
        (if (`KismetArrayLibrary.Array_IsValidIndex` (`self.NPCList`))
          (if (and (`KismetSystemLibrary.IsValidClass` _npcclass) (> _spawnamount 0))
            (set `self.CurrentNPC` (`|GetArrayItem` (`self.NPCList`) (`self.NPCIndex`)))
            (set `self.TotalNPCSpawns` (- (`.SpawnAmount_6_B84592A944E718473C2E548C4B7D88EF` (break `/Game/VV/SubSystems/NPCSystemV5/Data/Structs/POI/S_POI_NPCs` (`self.CurrentNPC`))) 1))
            (`|ExecutionSequence` :!label _label
              (:`then_0`
                (bind _returnvalue_2 (`|SpawnActorFromClass` (`.NPCClass_3_1430E86C4AE8E2A1E00E80B20F804FFD` (break `/Game/VV/SubSystems/NPCSystemV5/Data/Structs/POI/S_POI_NPCs` (`self.CurrentNPC`))) (`KismetMathLibrary.MakeTransform` (`KismetMathLibrary.RandomPointInBoundingBox` (`SceneComponent.K2_GetComponentLocation` _area) (`BoxComponent.GetScaledBoxExtent` _area)) (`self.K2_GetActorRotation`)) "AdjustIfPossibleButAlwaysSpawn" "OverrideRootScale" null null))
                (set `self.SpawnedNPC` _returnvalue_2)
                (`KismetArrayLibrary.Array_Add` (`self.SpawnedNPCs`) (`self.SpawnedNPC`)))
              (:`then_1`
                (`/Engine/EditorBlueprintResources/StandardMacros.IsValid` _returnvalue
                  (:`Is Valid`
                    (set `self.NPCController` _returnvalue)
                    (set `/Game/VV/SubSystems/NPCSystemV5/Blueprints/Characters/NPC/GenericAI/BPC_NPCController.ExecuteTaskOnStart` false (`self.NPCController`))
                    (set `/Game/VV/SubSystems/NPCSystemV5/Blueprints/Characters/NPC/GenericAI/BPC_NPCController.NPCManager` (`self.NPCManager`) (`self.NPCController`))
                    (set `/Game/VV/SubSystems/NPCSystemV5/Blueprints/Characters/NPC/GenericAI/BPC_NPCController.TargetPOI` self (`self.NPCController`))
                    (`|ExecutionSequence`
                      (:`then_0`
                        (bind _ascharacter (cast `Character` (`self.SpawnedNPC`)))
                        (`MovementComponent.StopMovementImmediately` (`Character.CharacterMovement` _ascharacter)))
                      (:`then_1`
                        (set `/Game/VV/SubSystems/NPCSystemV5/Blueprints/Characters/NPC/GenericAI/BPC_NPCController.NPC_State` "NewEnumerator0" (`self.NPCController`))
                        (`KismetSystemLibrary.Delay` 0.2)
                        (`|ExecutionSequence`
                          (:`then_0`
                            (`/Engine/EditorBlueprintResources/StandardMacros.IsValid` (`self.NPCController`)
                              (:`Is Valid`
                                (message `/Game/VV/SubSystems/NPCSystemV5/Blueprints/Interfaces/BPI_NPC_Controller.ArrivedAtPOI` (`self.DefaultSceneRoot`) self))))
                          (:`then_1`
                            (if (>= (`self.NPCSpawnCounter`) (`self.TotalNPCSpawns`))
                              (set `self.NPCSpawnCounter` 0)
                              (if (< (`self.NPCIndex`) (`KismetArrayLibrary.Array_LastIndex` (`self.NPCList`)))
                                (`/Engine/EditorBlueprintResources/StandardMacros.IncrementInt` (`self.NPCIndex`)
                                  (:`  `
                                    (`KismetSystemLibrary.Delay` (`KismetMathLibrary.RandomFloatInRange` 0.0 0.3))
                                    (`self.Ev_SpawnNPCs`)))
                                (else
                                  (set `self.NPCIndex` 0)
                                  (set `self.NPCsSpawned` true)))
                              (else
                                (`/Engine/EditorBlueprintResources/StandardMacros.IncrementInt` (`self.NPCSpawnCounter`)
                                  (:`  `
                                    (`KismetSystemLibrary.Delay` (`KismetMathLibrary.RandomFloatInRange` 0.0 0.2))
                                    (goto _label)))))))))))))))))))

(event `Ev_ShowHideProps`
  (params (`Show?` :type Boolean))
  (`self.Ev_ShowHideProps_MC` `Show?`))

(event `Ev_ShowHideProps_MC`
  (params (`Show?` :type Boolean))
  (`self.Fn_ShowHideProps` `Show?`))

(event `1_PopulateElements`
  (`self.Fn_PopulateElements`)
  (`self.Fn_ConfigureElements`))

(event `2_CategorizeStations`
  (`self.Fn_CategorizeElements`))

(event `self.ReceiveBeginPlay`
  (`self.Fn_SetStationMap`)
  (`|ExecutionSequence`
    (:`then_0`
      ;[0 0 0] Not spawn in the player proximity?
      (if (not (`self.SpawnOnPlayerProximity?`))
        (`KismetSystemLibrary.Delay` (`KismetMathLibrary.RandomFloatInRange` 0.0 0.2))
        ;[0 0 0] Spawn NOT on proximity
        (`self.Ev_SpawnNPCs`)))
    (:`then_1`
      (if (`self.HideStationProps?`)
        (`self.Ev_ShowHideProps` false)))))

(event `self.PlayerTrigger.OnComponentBeginOverlap`
  (params (OverlappedComponent :type "PrimitiveComponent Object Reference") (OtherActor :type "Actor Object Reference") (OtherComp :type "PrimitiveComponent Object Reference") (OtherBodyIndex :type Integer) (bFromSweep :type Boolean) (SweepResult :type "HitResult Structure (by ref)"))
  (if (and (`self.ActorHasTag` OtherActor "Player") (`self.HasAuthority` OtherActor))
    (`/Engine/EditorBlueprintResources/StandardMacros.DoOnce` false :!label _label_2
      (:`Completed`
        (`|ExecutionSequence`
          (:`then_0`
            ;[0 0 0] Spawn on Proximity
            (if (`self.SpawnOnPlayerProximity?`)
              (`self.Ev_SpawnNPCs`)))
          (:`then_1`
            (if (`self.HideStationProps?`)
              (`self.Ev_ShowHideProps` false))))))))

(event `self.PlayerTrigger.OnComponentEndOverlap`
  (params (OverlappedComponent :type "PrimitiveComponent Object Reference") (OtherActor :type "Actor Object Reference") (OtherComp :type "PrimitiveComponent Object Reference") (OtherBodyIndex :type Integer))
  (if (and (`self.ActorHasTag` OtherActor "Player") (`self.HasAuthority` OtherActor))
    (`|ExecutionSequence`
      (:`then_0`
        (goto _label_2 :!via `Reset`))
      (:`then_1`
        ;[0 0 0] Despawn on Proximity
        (if (`self.DespawnOnPlayerProximity?`)
          (`KismetSystemLibrary.Delay` 1.0)
          (if (not (`self.Fn_TraceForPlayers`))
            (set `self.NPCsSpawned` false)
            (`self.Fn_DespawnNPCs`))))
      (:`then_2`
        (if (`self.HideStationProps?`)
          (`self.Ev_ShowHideProps` false))))))

(fn `Fn_AssignStation`
  (params (Requestor :type "Actor Object Reference") (CurrentStation :type "/Game/VV/SubSystems/NPCSystemV5/Blueprints/Stations/BaseClasses/BP_Station_Base Object Reference") (NPCTagList :type "Array of Name") (ProfileTagList :type "Array of Name"))
  (returns (`FreeStationFound?` :type Boolean) (Station :type "/Game/VV/SubSystems/NPCSystemV5/Blueprints/Stations/BaseClasses/BP_Station_Base Object Reference"))
  (locals (NPC :type "Actor Object Reference") (CStation :type "/Game/VV/SubSystems/NPCSystemV5/Blueprints/Stations/BaseClasses/BP_Station_Base Object Reference") (NPCTList :type "Array of Name") (ProfileTList :type "Array of Name") (`StationFound?` :type Boolean) (LStation :type "/Game/VV/SubSystems/NPCSystemV5/Blueprints/Stations/BaseClasses/BP_Station_Base Object Reference") (Tag :type Name))
  (bind _freestation (`self.FreeStation`))
  (bind _returnvalue (`self.GetComponentByClass` (`local.NPC`) "/Game/VV/SubSystems/NPCSystemV5/Blueprints/Characters/NPC/GenericAI/BPC_NPCController.BPC_NPCController_C"))
  (bind _returnvalue_2 (`self.GetComponentByClass` (`local.NPC`) "/Game/VV/SubSystems/NPCSystemV5/Blueprints/Characters/NPC/GenericAI/BPC_NPCController.BPC_NPCController_C"))
  (set `local.NPC` Requestor)
  (set `local.CStation` CurrentStation)
  (set `local.NPCTList` NPCTagList)
  (set `local.ProfileTList` ProfileTagList)
  (`|ExecutionSequence`
    (:`then_0`
      (`|ExecutionSequence`
        (:`then_0`
          ;[0 0 0] If we dont have any free stations?
          (if (not (`KismetArrayLibrary.Array_IsValidIndex` (`self.FreeStation`)))
            ;[0 0 0] Loop through all the stations
            (bind _keys (`BlueprintMapLibrary.Map_Keys` (`self.RegularStationMap`)))
            (for _array_element _keys
              (bind _output_get (set `local.LStation` _array_element))
              (`/Engine/EditorBlueprintResources/StandardMacros.IsValid` _output_get
                (:`Is Valid`
                  ;[0 0 0] Check if the station is not being used
                  (if (not (`BlueprintMapLibrary.Map_Find` (`self.RegularStationMap`) (`local.LStation`)))
                    ;[0 0 0] Check if the station have the NPC's tag ?
                    (for _array_element_2 (`/Game/VV/SubSystems/NPCSystemV5/Blueprints/Stations/BaseClasses/BP_Station_Base.TagList` (`local.LStation`))
                      (set `local.Tag` _array_element_2)
                      (if (`KismetArrayLibrary.Array_Contains` (`local.NPCTList`) (`local.Tag`))
                        (if (`KismetArrayLibrary.Array_IsValidIndex` (`local.ProfileTList`))
                          ;[0 0 0] Check if the profile also have the NPC's tag ?
                          (if (`KismetArrayLibrary.Array_Contains` (`local.ProfileTList`) (`local.Tag`))
                            ;[0 0 0] Station is not one time use?
                            (if (not (`KismetArrayLibrary.Array_Contains` (`self.UnavailableStations`) (`local.LStation`))) :!label _label
                              ;[0 0 0] Add station to the free station list
                              (`KismetArrayLibrary.Array_Add` (`self.FreeStation`) (`local.LStation`))
                              (break)))
                          (else
                            (goto _label)))))))))))
        (:`then_1`
          ;[0 0 0] If we have any free stations?
          (if (`KismetArrayLibrary.Array_IsValidIndex` (`self.FreeStation`))
            ;[0 0 0] Possibility to assign the station to the NPC
            (if (`self.Fn_Helper_PossibilityCheck` (`self.PrecentChangeToAssignStation`))
              ;[0 0 0] Select a random free station
              (set `self.SelectedStation` (`|GetArrayItem` _freestation (`KismetMathLibrary.RandomIntegerInRange` 0 (`KismetArrayLibrary.Array_LastIndex` _freestation))))
              (else
                ;[0 0 0] Dont assign a station
                (set `self.SelectedStation` null)
                (set `local.StationFound?` false)))
            (`/Engine/EditorBlueprintResources/StandardMacros.IsValid` (`local.CStation`) :!label _label_2
              (:`Is Valid`
                (if (not (`KismetArrayLibrary.Array_Contains` (`self.UnavailableStations`) (`local.CStation`)))
                  (`BlueprintMapLibrary.Map_Add` (`self.StationAssignments`) (`local.CStation`))
                  (`BlueprintMapLibrary.Map_Add` (`self.RegularStationMap`) (`local.CStation`))))
              (:`Is Not Valid`
                _))
            (`BlueprintMapLibrary.Map_Add` (`self.RegularStationMap`) (`self.SelectedStation`) true)
            (set `local.StationFound?` true)
            (else
              ;[0 0 0] Possibility to assign the station to the NPC
              (if (`self.Fn_Helper_PossibilityCheck` (`self.PrecentChangeToAssignStation`))
                ;[0 0 0] Station is valid and not a one time use only?
                (if (and (`KismetSystemLibrary.IsValid` (`local.CStation`)) (not (`KismetArrayLibrary.Array_Contains` (`self.UnavailableStations`) (`local.CStation`))))
                  (set `self.SelectedStation` (`local.CStation`))
                  (else
                    (set `local.StationFound?` false :!label _label_3)
                    (goto _label_2)))
                (else
                  (goto _label_3))))))))
    (:`then_1`
      (`|ExecutionSequence`
        (:`then_0`
          (`/Engine/EditorBlueprintResources/StandardMacros.IsValid` (`self.SelectedStation`)
            (:`Is Valid`
              (`/Engine/EditorBlueprintResources/StandardMacros.IsValid` _returnvalue_2
                (:`Is Valid`
                  (`BlueprintMapLibrary.Map_Add` (`self.StationAssignments`) (`self.SelectedStation`) (`.NPCName_24_8EFD836B499B63370EA392B7421A1CE3` (break `/Game/VV/SubSystems/NPCSystemV5/Data/Structs/NPCController/S_NPCC_GeneralSettings` (`/Game/VV/SubSystems/NPCSystemV5/Blueprints/Characters/NPC/GenericAI/BPC_NPCController.GeneralSettings` _returnvalue_2)))))))))
        (:`then_1`
          (if (`self.DebugStationAssignment`)
            (`/Engine/EditorBlueprintResources/StandardMacros.IsValid` _returnvalue
              (:`Is Valid`
                (`KismetSystemLibrary.PrintString` (`KismetTextLibrary.Conv_TextToString` (`|FormatText` "{NPCName} - From [{currentStation}] to [{selectedStation}]" (`.NPCName_24_8EFD836B499B63370EA392B7421A1CE3` (break `/Game/VV/SubSystems/NPCSystemV5/Data/Structs/NPCController/S_NPCC_GeneralSettings` (`/Game/VV/SubSystems/NPCSystemV5/Blueprints/Characters/NPC/GenericAI/BPC_NPCController.GeneralSettings` _returnvalue))) (`KismetSystemLibrary.GetDisplayName` (`local.CStation`)) (`KismetSystemLibrary.GetDisplayName` (`self.SelectedStation`)))))))))))
    (:`then_2`
      ;[0 0 0] Return the selected station
      (return (`local.StationFound?`) (`self.SelectedStation`)))))

(fn `Fn_CategorizeElements`
  (`|ExecutionSequence`
    (:`then_0`
      ;[0 0 0] Mark Current Stations as free
      (for _array_element (`self.RegularStationList`)
        (`BlueprintMapLibrary.Map_Add` (`self.RegularStationMap`) _array_element)))))

(fn `Fn_ConfigureElements`
  (for _array_element (`self.EntranceList`)
    (set `/Game/VV/SubSystems/NPCSystemV5/Blueprints/POIs/BaseClasses/BP_POI_Entrance_Base.ParentPOI` self _array_element)))

(fn `Fn_DespawnNPCs`
  (locals (NPC :type "Actor Object Reference"))
  (bind _returnvalue (`self.GetComponentByClass` (`local.NPC`) "/Game/VV/SubSystems/NPCSystemV5/Blueprints/Characters/NPC/GenericAI/BPC_NPCController.BPC_NPCController_C"))
  (bind _assignedstation (`/Game/VV/SubSystems/NPCSystemV5/Blueprints/Characters/NPC/GenericAI/BPC_NPCController.AssignedStation` _returnvalue))
  (for _array_element (`self.SpawnedNPCs`)
    (bind _output_get (set `local.NPC` _array_element))
    (`/Engine/EditorBlueprintResources/StandardMacros.IsValid` _output_get
      (:`Is Valid`
        (`|ExecutionSequence`
          (:`then_0`
            ;[0 0 0] Free NPC's current station
            (`/Engine/EditorBlueprintResources/StandardMacros.IsValid` _returnvalue
              (:`Is Valid`
                (`/Engine/EditorBlueprintResources/StandardMacros.IsValid` _assignedstation
                  (:`Is Valid`
                    (if (not (`KismetArrayLibrary.Array_Contains` (`self.UnavailableStations`) _assignedstation))
                      (`self.Fn_SetStationFree` _assignedstation)
                      (set `/Game/VV/SubSystems/NPCSystemV5/Blueprints/Stations/BaseClasses/BP_Station_Base.StationOccupied?` false _assignedstation)))))))
          (:`then_1`
            (`self.K2_DestroyActor` (`local.NPC`))))))))

(fn `Fn_GetEntrance`
  (params (NPC :type "Actor Object Reference"))
  (returns (Entrance :type "Actor Object Reference"))
  (locals (E :type "/Game/VV/SubSystems/NPCSystemV5/Blueprints/POIs/BaseClasses/BP_POI_Entrance_Base Object Reference") (Actor :type "Actor Object Reference") (Distances :type "Array of Float (double-precision)"))
  (set `local.Actor` NPC)
  ;[0 0 0] Loop through all the entrances
  (for _array_element (`self.EntranceList`)
    (set `local.E` _array_element)
    ;[0 0 0] Add entrance distance to the array
    (`KismetArrayLibrary.Array_Add` (`local.Distances`) (`self.GetSquaredDistanceTo` (`local.E`) (`local.Actor`))))
  ;[0 0 0] Has at least 1 valid entrance?
  (if (`KismetArrayLibrary.Array_IsValidIndex` (`local.Distances`))
    ;[0 0 0] Get the closest entrance to the NPC
    (return (`|GetArrayItem` (`self.EntranceList`) (`KismetMathLibrary.MinOfFloatArray` (`local.Distances`))))
    (else
      (return null))))

(fn `Fn_Helper_PossibilityCheck`
  (params (Precentage :type "Float (double-precision)"))
  (returns (`Yes/No?` :type Boolean))
  (return (>= (`KismetMathLibrary.FClamp` Precentage) (`KismetMathLibrary.RandomFloatInRange` 0.0 1.0))))

(fn `Fn_Helper_VerifyActorOverClass`
  (params (Actor :type "Actor Object Reference") (Class :type "Actor Class Reference"))
  (returns (`Yes/No` :type Boolean))
  (return (or (`KismetMathLibrary.ClassIsChildOf` (`GameplayStatics.GetObjectClass` Actor) Class) (== (`GameplayStatics.GetObjectClass` Actor) Class))))

(fn `Fn_PopulateElements`
  (locals (HitActor :type "Actor Object Reference") (Station :type "/Game/VV/SubSystems/NPCSystemV5/Blueprints/Stations/BaseClasses/BP_Station_Base Object Reference"))
  (bind _returnvalue (`SceneComponent.K2_GetComponentLocation` (`self.Area`)))
  (`KismetArrayLibrary.Array_Clear` (`self.RegularStationList`))
  (`KismetArrayLibrary.Array_Clear` (`self.EntranceList`))
  (`KismetArrayLibrary.Array_Clear` (`self.SpawnPoints`))
  (`BlueprintMapLibrary.Map_Clear` (`self.RegularStationMap`))
  ;[0 0 0] Trace for stations/entrances/spawners
  (bind _outhits (`KismetSystemLibrary.BoxTraceMultiForObjects` _returnvalue (+ _returnvalue (0.0 0.0 0.01)) (`BoxComponent.GetScaledBoxExtent` (`self.Area`)) (`self.K2_GetActorRotation`) (`|MakeArray` "ObjectTypeQuery7" :!type "EObjectTypeQuery Enum")))
  (for _array_element _outhits
    (set `local.HitActor` (`.HitActor` (`GameplayStatics.BreakHitResult` _array_element)))
    (`|ExecutionSequence`
      (:`then_0`
        ;[0 0 0] Is a Station?
        (if (`self.Fn_Helper_VerifyActorOverClass` (`local.HitActor`) "/Game/VV/SubSystems/NPCSystemV5/Blueprints/Stations/BaseClasses/BP_Station_Base.BP_Station_Base_C")
          (bind _asbp_station_base (cast `/Game/VV/SubSystems/NPCSystemV5/Blueprints/Stations/BaseClasses/BP_Station_Base` (`local.HitActor`)))
          (set `local.Station` _asbp_station_base)
          ;[0 0 0] Add to List
          (`KismetArrayLibrary.Array_AddUnique` (`self.RegularStationList`) (`local.Station`))))
      (:`then_1`
        ;[0 0 0] Is a Entrance?
        (if (`self.Fn_Helper_VerifyActorOverClass` (`local.HitActor`) "/Game/VV/SubSystems/NPCSystemV5/Blueprints/POIs/BaseClasses/BP_POI_Entrance_Base.BP_POI_Entrance_Base_C")
          ;[0 0 0] Add to list
          (bind _asbp_poi_entrance_base (cast `/Game/VV/SubSystems/NPCSystemV5/Blueprints/POIs/BaseClasses/BP_POI_Entrance_Base` (`local.HitActor`)))
          (`KismetArrayLibrary.Array_AddUnique` (`self.EntranceList`) _asbp_poi_entrance_base)))
      (:`then_2`
        ;[0 0 0] Is a Spawner?
        (if (`self.Fn_Helper_VerifyActorOverClass` (`local.HitActor`) "/Game/VV/SubSystems/NPCSystemV5/Blueprints/POIs/BaseClasses/BP_POI_NPCSpawner.BP_POI_NPCSpawner_C")
          ;[0 0 0] Add to List
          (bind _asbp_poi_npcspawner (cast `/Game/VV/SubSystems/NPCSystemV5/Blueprints/POIs/BaseClasses/BP_POI_NPCSpawner` (`local.HitActor`)))
          (`KismetArrayLibrary.Array_AddUnique` (`self.SpawnPoints`) _asbp_poi_npcspawner))))))

(fn `Fn_SetStationFree`
  (params (Station :type "/Game/VV/SubSystems/NPCSystemV5/Blueprints/Stations/BaseClasses/BP_Station_Base Object Reference"))
  (locals (CurrentStation :type "/Game/VV/SubSystems/NPCSystemV5/Blueprints/Stations/BaseClasses/BP_Station_Base Object Reference"))
  (set `local.CurrentStation` Station)
  (`|ExecutionSequence`
    (:`then_0`
      ;[0 0 0] Mark station as free
      (`BlueprintMapLibrary.Map_Add` (`self.RegularStationMap`) (`local.CurrentStation`)))))

(fn `Fn_SetStationMap`
  ;[0 0 0] Mark current stations as free
  (for _array_element (`self.RegularStationList`)
    (`BlueprintMapLibrary.Map_Add` (`self.RegularStationMap`) _array_element)))

(fn `Fn_SetStationUnavailable`
  (params (Station :type "/Game/VV/SubSystems/NPCSystemV5/Blueprints/Stations/BaseClasses/BP_Station_Base Object Reference (by ref)"))
  (`KismetArrayLibrary.Array_AddUnique` (`self.UnavailableStations`) Station))

(fn `Fn_ShowHideProps`
  (params (`Show?` :type Boolean))
  (`|ExecutionSequence`
    (:`then_0`
      (for _array_element (`self.RegularStationList`)
        (message `/Game/VV/SubSystems/NPCSystemV5/Blueprints/Interfaces/BPI_Station.ShowHideProps` _array_element `Show?`)))))

(fn `Fn_TraceForPlayers`
  (returns (`FoundPlayer?` :type Boolean))
  (locals (`Found?` :type Boolean :default false))
  (bind _playertrigger (`self.PlayerTrigger`))
  (bind _returnvalue (`SceneComponent.K2_GetComponentLocation` _playertrigger))
  ;[0 0 0] Trace for pawns within the player trigger
  (bind (_outhits _returnvalue_2) (`KismetSystemLibrary.BoxTraceMultiForObjects` _returnvalue (+ _returnvalue (0.0 0.0 0.001)) (`.BoxExtent` (`KismetSystemLibrary.GetComponentBounds` _playertrigger)) (`SceneComponent.K2_GetComponentRotation` _playertrigger) (`|MakeArray` "ObjectTypeQuery3" :!type "EObjectTypeQuery Enum")))
  ;[0 0 0] Check pawn is a player?
  (if _returnvalue_2
    (for _array_element _outhits
      (if (`self.ActorHasTag` (`.HitActor` (`GameplayStatics.BreakHitResult` _array_element)) "Player")
        (set `local.Found?` false)
        (break)))
    (return (`local.Found?`))))

(fn `UserConstructionScript`
  (bind (_areascale _playertriggerscale) (break `/Game/VV/SubSystems/NPCSystemV5/Data/Structs/POI/S_POI_GeneralSettings` (`self.GeneralSettings`)))
  ;[0 0 0] Trigger scales
  (`SceneComponent.SetWorldScale3D` (`self.Area`) _areascale)
  (`SceneComponent.SetWorldScale3D` (`self.PlayerTrigger`) _playertriggerscale))