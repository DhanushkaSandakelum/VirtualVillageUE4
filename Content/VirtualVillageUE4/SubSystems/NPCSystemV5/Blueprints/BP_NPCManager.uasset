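; BP_NPCManager is the central manager for the NPC system, holding registries of NPCs and points of interest.
; On BeginPlay, the authority collects every BP_POI_Base actor into a map keyed by class and gives each a back-reference to the manager.
; Because the key is the class, the map keeps only one POI per class.
; It also exposes functions to register NPCs and read the current hour from a day-cycle Blueprint.
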(event `self.ReceiveBeginPlay`
  (`/Engine/EditorBlueprintResources/ActorMacros.Switch Has Authority`
    (:`Authority`
      (`self.Fn_GetAllPOIs`))))

(fn `Fn_GetAllPOIs`
  (locals (POI :type "/Game/VirtualVillageUE4/SubSystems/NPCSystemV5/Blueprints/POIs/BaseClasses/BP_POI_Base Object Reference"))
  (`BlueprintMapLibrary.Map_Clear` (`self.POIMap`))
  ;[0 0 0] Loop through all the POIs in the map
  (bind _outactors (`GameplayStatics.GetAllActorsOfClass` "/Game/VirtualVillageUE4/SubSystems/NPCSystemV5/Blueprints/POIs/BaseClasses/BP_POI_Base.BP_POI_Base_C"))
  (for _array_element _outactors
    (set `local.POI` _array_element)
    ;[0 0 0] Add POI to the map
    (`BlueprintMapLibrary.Map_Add` (`self.POIMap`) (`GameplayStatics.GetObjectClass` (`local.POI`)) (`local.POI`))
    (set `/Game/VirtualVillageUE4/SubSystems/NPCSystemV5/Blueprints/POIs/BaseClasses/BP_POI_Base.NPCManager` self (`local.POI`))))

(fn `Fn_GetTimeOfDay`
  (returns (`Found?` :type Boolean) (CurrentHour :type "Float (double-precision)"))
  (`/Engine/EditorBlueprintResources/StandardMacros.IsValid` (`self.DayCycleBP`)
    (:`Is Valid`
      (return true (`self.CurrentHour`)))
    (:`Is Not Valid`
      (return false 0.0))))

(fn `Fn_RegisterNPC`
  (params (NPC :type "Actor Object Reference (by ref)"))
  (`KismetArrayLibrary.Array_Add` (`self.NPCList`) NPC))

(fn `UserConstructionScript`)