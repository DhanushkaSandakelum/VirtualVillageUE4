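; Base point-of-interest entrance actor for the NPC system, signalling when an NPC arrives at its parent POI.
; When an actor carrying an NPC controller component overlaps the trigger, it sends an arrival message through the NPC controller interface, passing the parent POI.
; The construction script sets the entrance component's editor and in-game visibility from variables.
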(event `self.Trigger.OnComponentBeginOverlap`
  (params (OverlappedComponent :type "PrimitiveComponent Object Reference") (OtherActor :type "Actor Object Reference") (OtherComp :type "PrimitiveComponent Object Reference") (OtherBodyIndex :type Integer) (bFromSweep :type Boolean) (SweepResult :type "HitResult Structure (by ref)"))
  (bind _returnvalue (`self.GetComponentByClass` (`self.OverlappedActor`) "/Game/VirtualVillageUE4/SubSystems/NPCSystemV5/Blueprints/Characters/NPC/GenericAI/BPC_NPCController.BPC_NPCController_C"))
  (set `self.OverlappedActor` OtherActor)
  (`/Engine/EditorBlueprintResources/StandardMacros.IsValid` _returnvalue
    (:`Is Valid`
      (bind _output_get (set `self.NPCController` _returnvalue))
      (if (`KismetSystemLibrary.DoesImplementInterface` _output_get "/Game/VirtualVillageUE4/SubSystems/NPCSystemV5/Blueprints/Interfaces/BPI_NPC_Controller.BPI_NPC_Controller_C")
        (message `/Game/VirtualVillageUE4/SubSystems/NPCSystemV5/Blueprints/Interfaces/BPI_NPC_Controller.ArrivedAtPOI` (`self.NPCController`) (`self.ParentPOI`))))))

(fn `UserConstructionScript`
  ;[0 0 0] Visibilities
  (`SceneComponent.SetVisibility` (`self.Entrance`) (`self.EntranceVisible?`) false)
  (`SceneComponent.SetHiddenInGame` (`self.Entrance`) (`self.EntranceHidden?`) false))