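; Component controller for spline crowd NPCs that handles tick optimization and temporary collision changes on its owning Character.
; On BeginPlay it caches the owner and, if Active, calls FnOptimizeNPC, which disables the owner's actor tick.
; A separate Ev_ChangeCollision event makes the capsule ignore the Pawn channel, then restores blocking after a short delay, briefly letting pawns pass through.
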(event `self.ReceiveBeginPlay`
  (bind _ascharacter (cast `Character` (`self.GetOwner`)))
  (set `self.Owner` _ascharacter)
  (if (`self.Active?`)
    (`self.Fn_OptimizeNPC`)))

(event `Ev_ChangeCollision`
  (bind _ascharacter (cast `Character` (`self.GetOwner`)))
  (`PrimitiveComponent.SetCollisionResponseToChannel` (`Character.CapsuleComponent` _ascharacter) "ECC_Pawn" "ECR_Ignore")
  (`KismetSystemLibrary.Delay` 0.5)
  (bind _ascharacter_2 (cast `Character` (`self.GetOwner`)))
  (`PrimitiveComponent.SetCollisionResponseToChannel` (`Character.CapsuleComponent` _ascharacter_2) "ECC_Pawn" "ECR_Block"))

(fn `Fn_OptimizeNPC`
  (`Actor.SetActorTickEnabled` (`self.Owner`) false))