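; Spline crowd intersection that lets crowd NPCs randomly switch between overlapping spline paths.
; An editor event box-traces the trigger volume to cache the BP_SplineCrowd paths it touches.
; When a character tagged SplineCrowd enters the trigger, a probability roll decides whether it leaves its current path's NPC list and joins a random other cached path.
; The construction script applies trigger scale and visibility settings.
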(event `self.Trigger.OnComponentBeginOverlap`
  (params (OverlappedComponent :type "PrimitiveComponent Object Reference") (OtherActor :type "Actor Object Reference") (OtherComp :type "PrimitiveComponent Object Reference") (OtherBodyIndex :type Integer) (bFromSweep :type Boolean) (SweepResult :type "HitResult Structure (by ref)"))
  (if (`self.ActorHasTag` OtherActor "SplineCrowd")
    (bind _ascharacter (cast `Character` OtherActor))
    (set `self.OverlappedActor` _ascharacter)
    (`self.Fn_ChangePaths`)))

(event `1_PopulateSplinePathList`
  (bind _returnvalue (`SceneComponent.K2_GetComponentLocation` (`self.Trigger`)))
  (`KismetArrayLibrary.Array_Clear` (`self.SplinePathList`))
  ;[0 0 0] Trace for paths
  (bind _outhits (`KismetSystemLibrary.BoxTraceMultiForObjects` _returnvalue (+ _returnvalue (0.0 0.0 0.01)) (`BoxComponent.GetScaledBoxExtent` (`self.Trigger`)) (`self.K2_GetActorRotation`) (`|MakeArray` "ObjectTypeQuery7" :!type "EObjectTypeQuery Enum")))
  (for _array_element _outhits
    (set `self.HitActor` (`.HitActor` (`GameplayStatics.BreakHitResult` _array_element)))
    (bind _asbp_spline_crowd (cast `/Game/VirtualVillageUE4/SubSystems/NPCSystemV5/Blueprints/Characters/NPC/CrowdAI/SplineCrowd/BP_SplineCrowd` (`self.HitActor`)))
    (`KismetArrayLibrary.Array_AddUnique` (`self.SplinePathList`) _asbp_spline_crowd)))

(fn `Fn_ChangePaths`
  (locals (TempList :type "Array of /Game/VirtualVillageUE4/SubSystems/NPCSystemV5/Blueprints/Characters/NPC/CrowdAI/SplineCrowd/BP_SplineCrowd Object Reference") (Path :type "/Game/VirtualVillageUE4/SubSystems/NPCSystemV5/Blueprints/Characters/NPC/CrowdAI/SplineCrowd/BP_SplineCrowd Object Reference") (Index :type Integer))
  (bind _splinepathlist (`self.SplinePathList`))
  (bind _templist (`local.TempList`))
  (if (`self.Fn_Helper_PossibilityCheck` (`self.PercentChanceToSwitch`))
    (set `local.TempList` _splinepathlist)
    (if (>= (`KismetArrayLibrary.Array_Length` _splinepathlist) 2)
      (for (_array_element _array_index) (`local.TempList`)
        (set `local.Path` _array_element)
        (set `local.Index` _array_index)
        ;[0 0 0] NPC is a part of a path?
        (if (`KismetArrayLibrary.Array_Contains` (`/Game/VirtualVillageUE4/SubSystems/NPCSystemV5/Blueprints/Characters/NPC/CrowdAI/SplineCrowd/BP_SplineCrowd.NPCList` (`local.Path`)) (`self.OverlappedActor`))
          ;[0 0 0] Remove the NPC
          (`KismetArrayLibrary.Array_RemoveItem` (`/Game/VirtualVillageUE4/SubSystems/NPCSystemV5/Blueprints/Characters/NPC/CrowdAI/SplineCrowd/BP_SplineCrowd.NPCList` (`local.Path`)) (`self.OverlappedActor`))
          ;[0 0 0] Remove path
          (`KismetArrayLibrary.Array_RemoveItem` (`local.TempList`) (`local.Path`))))
      (`KismetArrayLibrary.Array_Add` (`/Game/VirtualVillageUE4/SubSystems/NPCSystemV5/Blueprints/Characters/NPC/CrowdAI/SplineCrowd/BP_SplineCrowd.NPCList` (`|GetArrayItem` _templist (`KismetMathLibrary.RandomIntegerInRange` 0 (`KismetArrayLibrary.Array_LastIndex` _templist)))) (`self.OverlappedActor`)))))

(fn `Fn_Helper_PossibilityCheck`
  (params (Precentage :type "Float (double-precision)"))
  (returns (`Yes/No?` :type Boolean))
  (return (>= (`KismetMathLibrary.FClamp` Precentage) (`KismetMathLibrary.RandomFloatInRange` 0.0 1.0))))

(fn `UserConstructionScript`
  (`SceneComponent.SetWorldScale3D` (`self.Trigger`) (`self.TriggerScale`))
  (`SceneComponent.SetVisibility` (`self.Trigger`) (`self.TriggerVisible?`) false)
  (`SceneComponent.SetHiddenInGame` (`self.Trigger`) (`self.TriggerHidden?`) false))