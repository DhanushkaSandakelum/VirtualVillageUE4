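; Crowd actor that spawns random NPCs along a spline with lateral offsets and varied walk speeds, then keeps them walking along it.
; Steering follows the spline direction or turns back when strayed, using per-tick movement input in single player and timer-updated blackboard targets in multiplayer.
; On open splines, NPCs nearing the end teleport to the start.
; An optional trigger defers spawning and hides and pauses the crowd without players inside.
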(event `Ev_TeleportNPC_Server`
  (params (NPC :type "Actor Object Reference"))
  (set `self.NPCActor` NPC)
  (set `self.TargetLocation` (`self.Fn_Helper_GetTeleportLocation`))
  (`self.Ev_TeleportNPC_MC` (`self.NPCActor`)))

(event `Ev_TeleportNPC_MC`
  (params (NPC :type "Actor Object Reference"))
  (`self.K2_SetActorLocationAndRotation` NPC (`self.TargetLocation`) (`SplineComponent.GetRotationAtSplinePoint` (`self.Spline`) 0 "World") false false))

(event `Ev_MoveNPCs`
  (`KismetSystemLibrary.K2_SetTimerDelegate` (delegate `Ev_MoveNPCs`) 1.0 true)
  (`/Engine/EditorBlueprintResources/ActorMacros.Switch Has Authority`
    (:`Authority`
      (if (`self.MoveNPCs?`)
        (`self.Fn_MoveNPCs`)))))

(event `Ev_EnableNPCs`
  (params (Enable :type Boolean))
  (`self.Fn_EnableNPCs` Enable))

(event `self.ReceiveBeginPlay`
  (if (`self.Active?`)
    (`/Engine/EditorBlueprintResources/ActorMacros.Switch Has Authority`
      (:`Authority`
        ;[0 0 0] Get NPC Tag
        (set `self.NPCTag` (`KismetStringLibrary.Conv_StringToName` (`KismetSystemLibrary.GetDisplayName` self)))
        (if (not (`self.UseTrigger?`))
          (`KismetSystemLibrary.Delay` (`KismetMathLibrary.RandomFloatInRange` 0.0 0.75))
          (`|ExecutionSequence`
            (:`then_0`
              (if (not (`self.SpawnedNPCs`))
                (`self.Fn_SpawnNPCs`)
                ;[0 0 0] If we using the Trigger, disable the NPCs
                (if (`self.UseTrigger?`)
                  (bind _found_player (`self.Fn_TraceForPlayers`))
                  (if (not _found_player)
                    (set `self.MoveNPCs?` false)
                    (`self.Fn_EnableNPCs` false)))))
            (:`then_1`
              (switch `/Game/VirtualVillageUE4/SubSystems/NPCSystemV5/Data/Enums/SplineCrowd/E_SplineCrowd_Mode` (`self.Mode`)
                (:`NewEnumerator1`
                  (`self.Ev_MoveNPCs`))))))))))

(event `self.ReceiveTick`
  (params (DeltaSeconds :type "Float (single-precision)"))
  (switch `/Game/VirtualVillageUE4/SubSystems/NPCSystemV5/Data/Enums/SplineCrowd/E_SplineCrowd_Mode` (`self.Mode`)
    (:`NewEnumerator0`
      ;[0 0 0] Move NPCs along the spline
      (if (`self.MoveNPCs?`)
        (`self.Fn_MoveNPCs`)))))

(event `self.Trigger.OnComponentBeginOverlap`
  (params (OverlappedComponent :type "PrimitiveComponent Object Reference") (OtherActor :type "Actor Object Reference") (OtherComp :type "PrimitiveComponent Object Reference") (OtherBodyIndex :type Integer) (bFromSweep :type Boolean) (SweepResult :type "HitResult Structure (by ref)"))
  (if (and (`self.ActorHasTag` OtherActor "Player") (`self.UseTrigger?`))
    (`/Engine/EditorBlueprintResources/ActorMacros.Switch Has Authority`
      (:`Authority`
        (if (not (`self.SpawnedNPCs`))
          (`self.Fn_SpawnNPCs`)
          (`KismetSystemLibrary.Delay` 0.2)
          (`self.Ev_MoveNPCs`))
        (set `self.MoveNPCs?` true)
        (`self.Ev_EnableNPCs` true)))))

(event `self.Trigger.OnComponentEndOverlap`
  (params (OverlappedComponent :type "PrimitiveComponent Object Reference") (OtherActor :type "Actor Object Reference") (OtherComp :type "PrimitiveComponent Object Reference") (OtherBodyIndex :type Integer))
  (if (and (`self.ActorHasTag` OtherActor "Player") (`self.UseTrigger?`))
    (`/Engine/EditorBlueprintResources/ActorMacros.Switch Has Authority`
      (:`Authority`
        (`KismetSystemLibrary.Delay` 2.0)
        (bind _found_player (`self.Fn_TraceForPlayers`))
        (if (not _found_player)
          (set `self.MoveNPCs?` false)
          (`self.Ev_EnableNPCs` false))))))

(fn `Fn_EnableNPCs`
  (params (Enable :type Boolean))
  (locals (NPC :type "Character Object Reference"))
  (if Enable
    (for _array_element (`self.NPCList`)
      (set `local.NPC` _array_element)
      (`self.SetActorHiddenInGame` (`local.NPC`) false)
      (`self.SetActorEnableCollision` (`local.NPC`) true))
    (else
      (for _array_element_2 (`self.NPCList`)
        (set `local.NPC` _array_element_2)
        (`self.SetActorHiddenInGame` (`local.NPC`) true)
        (`self.SetActorEnableCollision` (`local.NPC`) false)))))

(fn `Fn_Helper_GetRandomLocationAndRotation`
  (returns (Transform :type "Transform Structure"))
  (bind _randomdistance (`self.RandomDistance`))
  (bind _spline (`self.Spline`))
  (bind (_splineoffsetrange_x _splineoffsetrange_y) (`KismetMathLibrary.BreakVector2D` (`self.SplineOffsetRange`)))
  (bind _returnvalue (`SplineComponent.GetRotationAtDistanceAlongSpline` _spline _randomdistance "World"))
  (return (`KismetMathLibrary.MakeTransform` (+ (`SplineComponent.GetLocationAtDistanceAlongSpline` _spline _randomdistance "World") (* (`KismetMathLibrary.GetRightVector` _returnvalue) (`KismetMathLibrary.RandomFloatInRange` _splineoffsetrange_x _splineoffsetrange_y))) _returnvalue)))

(fn `Fn_Helper_GetTeleportLocation`
  (returns (Location :type "Vector Structure") (Rotation :type "Rotator Structure"))
  (bind _spline (`self.Spline`))
  (bind (_splineoffsetrange_x _splineoffsetrange_y) (`KismetMathLibrary.BreakVector2D` (`self.SplineOffsetRange`)))
  (bind _returnvalue (`SplineComponent.GetRotationAtSplinePoint` _spline 0 "World"))
  (return (+ (+ (+ (`SplineComponent.GetLocationAtSplinePoint` _spline 0 "World") (* (`KismetMathLibrary.GetForwardVector` _returnvalue) (`KismetMathLibrary.RandomFloatInRange` 1.0 (* _splineoffsetrange_y 2.0)))) (* (`KismetMathLibrary.GetForwardVector` _returnvalue) (`KismetMathLibrary.RandomFloatInRange` _splineoffsetrange_x _splineoffsetrange_y))) (0.0 0.0 100.0)) _returnvalue))

(fn `Fn_MoveNPCs`
  (locals (NPC :type "Character Object Reference") (NPCController :type "/Game/VirtualVillageUE4/SubSystems/NPCSystemV5/Blueprints/Characters/NPC/CrowdAI/SplineCrowd/BPC_NPC_SplineCrowd_Controller Object Reference") (Direction :type "Vector Structure" :default (0.0 0.0 0.0)))
  (bind _npc (`local.NPC`))
  (bind _npc_2 (`local.NPC`))
  (bind _spline (`self.Spline`))
  (bind (_splineoffsetrange_x _splineoffsetrange_y) (`KismetMathLibrary.BreakVector2D` (`self.SplineOffsetRange`)))
  (bind _returnvalue (`self.GetComponentByClass` (`local.NPC`) "/Game/VirtualVillageUE4/SubSystems/NPCSystemV5/Blueprints/Characters/NPC/CrowdAI/SplineCrowd/BPC_NPC_SplineCrowd_Controller.BPC_NPC_SplineCrowd_Controller_C"))
  (bind _returnvalue_2 (`self.K2_GetActorLocation` (`local.NPC`)))
  (bind _returnvalue_3 (`self.K2_GetActorLocation` (`local.NPC`)))
  (for _array_element (`self.NPCList`)
    (bind _output_get (set `local.NPC` _array_element))
    (`/Engine/EditorBlueprintResources/StandardMacros.IsValid` _output_get
      (:`Is Valid`
        (`/Engine/EditorBlueprintResources/StandardMacros.IsValid` _returnvalue
          (:`Is Valid`
            (set `local.NPCController` _returnvalue)
            ;[0 0 0] NPC Distances to the spline offset range
            (if (<= (`KismetMathLibrary.Vector_Distance2D` _returnvalue_2 (`SplineComponent.FindLocationClosestToWorldLocation` (`self.Spline`) _returnvalue_2 "World")) (select `bool` (< _splineoffsetrange_x _splineoffsetrange_y) :`false` _splineoffsetrange_x :`true` _splineoffsetrange_y))
              ;[0 0 0] Set direction
              (set `local.Direction` (`KismetMathLibrary.GetForwardVector` (`SplineComponent.FindRotationClosestToWorldLocation` (`self.Spline`) (`self.K2_GetActorLocation` (`local.NPC`)) "World")))
              ;[0 0 0] Add movement input along spline
              (switch `/Game/VirtualVillageUE4/SubSystems/NPCSystemV5/Data/Enums/SplineCrowd/E_SplineCrowd_Mode` (`self.Mode`)
                (:`NewEnumerator0`
                  (`Pawn.AddMovementInput` (`local.NPC`) (`local.Direction`) 1.0 false))
                (:`NewEnumerator1`
                  (`BlackboardComponent.SetValueAsVector` (`AIBlueprintHelperLibrary.GetBlackboard` _npc_2) "Location" (+ (`self.K2_GetActorLocation` _npc_2) (* (`local.Direction`) 500.0)))))
              (else
                ;[0 0 0] Set direction
                (set `local.Direction` (`KismetMathLibrary.GetForwardVector` (`KismetMathLibrary.FindLookAtRotation` _returnvalue_3 (`SplineComponent.FindLocationClosestToWorldLocation` (`self.Spline`) _returnvalue_3 "World"))))
                ;[0 0 0] Add movement input along spline
                (switch `/Game/VirtualVillageUE4/SubSystems/NPCSystemV5/Data/Enums/SplineCrowd/E_SplineCrowd_Mode` (`self.Mode`)
                  (:`NewEnumerator0`
                    (`Pawn.AddMovementInput` (`local.NPC`) (`local.Direction`) 1.0 false))
                  (:`NewEnumerator1`
                    (`BlackboardComponent.SetValueAsVector` (`AIBlueprintHelperLibrary.GetBlackboard` _npc) "Location" (+ (`self.K2_GetActorLocation` _npc) (* (`local.Direction`) 500.0)))))))
            (if (not (>= (`KismetMathLibrary.VSize` (`MovementComponent.Velocity` (`Character.CharacterMovement` (`local.NPC`)))) 1.0))
              (`/Game/VirtualVillageUE4/SubSystems/NPCSystemV5/Blueprints/Characters/NPC/CrowdAI/SplineCrowd/BPC_NPC_SplineCrowd_Controller.Ev_ChangeCollision` (`local.NPCController`)))
            (if (not (`self.ClosedLoop?`))
              ;[0 0 0] Check the spline distances and teleport distance
              (if (<= (`KismetMathLibrary.Vector_Distance2D` (`self.K2_GetActorLocation` (`local.NPC`)) (`SplineComponent.GetLocationAtSplinePoint` _spline (- (`SplineComponent.GetNumberOfSplinePoints` _spline) 1) "World")) (`self.TeleportDistance`))
                (`self.Ev_TeleportNPC_Server` (`local.NPC`))))))))))

(fn `Fn_SpawnNPCs`
  (locals (SpwnedNPC :type "Character Object Reference"))
  (bind (_speedmultiplierrange_x _speedmultiplierrange_y) (`KismetMathLibrary.BreakVector2D` (`self.SpeedMultiplierRange`)))
  (bind _npcclasses (`self.NPCClasses`))
  (bind _charactermovement (`Character.CharacterMovement` (`local.SpwnedNPC`)))
  (for _ (range (`self.TotalSpawns`))
    ;[0 0 0] Get random distance
    (set `self.RandomDistance` (`KismetMathLibrary.RandomFloatInRange` 0.0 (`SplineComponent.GetSplineLength` (`self.Spline`))))
    ;[0 0 0] Spawn random NPC
    (bind _returnvalue (`|SpawnActorFromClass` (`|GetArrayItem` _npcclasses (`KismetMathLibrary.RandomIntegerInRange` 0 (`KismetArrayLibrary.Array_LastIndex` _npcclasses))) (`self.Fn_Helper_GetRandomLocationAndRotation`) "AdjustIfPossibleButAlwaysSpawn" "OverrideRootScale" null null))
    (set `local.SpwnedNPC` _returnvalue)
    (switch `/Game/VirtualVillageUE4/SubSystems/NPCSystemV5/Data/Enums/SplineCrowd/E_SplineCrowd_Mode` (`self.Mode`)
      (:`NewEnumerator0`
        _)
      (:`NewEnumerator1`
        (bind _asbp_spline_crowd_aicontroller (cast `/Game/VirtualVillageUE4/SubSystems/NPCSystemV5/Blueprints/Characters/NPC/CrowdAI/SplineCrowd/AI/BP_SplineCrowd_AIController` (`AIBlueprintHelperLibrary.GetAIController` (`local.SpwnedNPC`))))
        (`/Game/VirtualVillageUE4/SubSystems/NPCSystemV5/Blueprints/Characters/NPC/CrowdAI/SplineCrowd/AI/BP_SplineCrowd_AIController.Ev_RunBT` _asbp_spline_crowd_aicontroller)))
    (`KismetArrayLibrary.Array_Add` (`Actor.Tags` (`local.SpwnedNPC`)) (`self.NPCTag`))
    (`KismetArrayLibrary.Array_Add` (`Actor.Tags` (`local.SpwnedNPC`)) "SplineCrowd")
    (`SkinnedMeshComponent.SetForcedLOD` (`Character.Mesh` (`local.SpwnedNPC`)) (`self.MeshForcedLOD`))
    ;[0 0 0] Set walk speed
    (set `CharacterMovementComponent.MaxWalkSpeed` (* (`CharacterMovementComponent.MaxWalkSpeed` _charactermovement) (`KismetMathLibrary.RandomFloatInRange` _speedmultiplierrange_x _speedmultiplierrange_y)) _charactermovement)
    (`KismetArrayLibrary.Array_Add` (`self.NPCList`) (`local.SpwnedNPC`)))
  (set `self.MoveNPCs?` true)
  (set `self.SpawnedNPCs` true))

(fn `Fn_TeleportNPC`
  (params (`NPC to Teleport` :type "Actor Object Reference"))
  (locals (NPC :type "Actor Object Reference") (Location :type "Vector Structure" :default (0.0 0.0 0.0)))
  (bind (_location _rotation) (`self.Fn_Helper_GetTeleportLocation`))
  (bind _output_get (set `local.NPC` `NPC to Teleport`))
  (set `local.Location` (`self.K2_GetActorLocation` _output_get))
  (`self.K2_SetActorLocationAndRotation` (`local.NPC`) _location _rotation false true))

(fn `Fn_TraceForPlayers`
  (returns (`Found Player` :type Boolean))
  (locals (Found :type Boolean :default false))
  (bind _trigger (`self.Trigger`))
  (bind _returnvalue (`SceneComponent.K2_GetComponentLocation` _trigger))
  (bind (_outhits _returnvalue_2) (`KismetSystemLibrary.BoxTraceMultiForObjects` _returnvalue (+ _returnvalue (0.0 0.0 0.01)) (`.BoxExtent` (`KismetSystemLibrary.GetComponentBounds` _trigger)) (`SceneComponent.RelativeRotation` _trigger) (`|MakeArray` "ObjectTypeQuery3" :!type "EObjectTypeQuery Enum")))
  ;[1 1 1] Check if we have a pawn called "Player"
  (if _returnvalue_2
    (for _array_element _outhits
      (if (`self.ActorHasTag` (`.HitActor` (`GameplayStatics.BreakHitResult` _array_element)) "Player")
        (set `local.Found` true)
        (break))))
  (return (`local.Found`)))

(fn `UserConstructionScript`)