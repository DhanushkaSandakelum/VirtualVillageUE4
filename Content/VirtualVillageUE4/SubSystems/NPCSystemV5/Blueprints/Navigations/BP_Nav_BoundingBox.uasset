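; Bounding-box helper actor for NPC navigation in NPCSystemV5, with no active runtime logic.
; The construction script enlarges the billboard, sizes Bounds from BoundsScale and scales Marker proportionally to it.
; It sets Marker visibility from MarkerVisible, then again from MarkerHidden, so the second call overrides the first.
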(fn `UserConstructionScript`
  (`SceneComponent.SetWorldScale3D` (`self.Billboard`) (5.0 5.0 5.0))
  (`SceneComponent.SetWorldScale3D` (`self.Bounds`) (`self.BoundsScale`))
  (`SceneComponent.SetWorldScale3D` (`self.Marker`) (* (`self.BoundsScale`) 0.625))
  (`SceneComponent.SetVisibility` (`self.Marker`) (`self.MarkerVisible?`) false)
  (`SceneComponent.SetVisibility` (`self.Marker`) (`self.MarkerHidden?`) false))