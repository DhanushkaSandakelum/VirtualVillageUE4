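; Base Blueprint for NPC stations in NPCSystemV5, marking a spot with an entry point, prop and preview pose.
; The construction script applies GeneralSettings to the area, nav mesh blocker, prop and pose skeleton, and BeginPlay stores the Arrow transform in StationOptions.
; An actor with BPC_NPCController entering the trigger receives an arrival message with that info, gated by a DoOnce that resets on exit.
; An interface event toggles prop visibility.
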(event `self.ReceiveBeginPlay`
  (bind (_returnvalue_location _returnvalue_rotation) (`KismetMathLibrary.BreakTransform` (`SceneComponent.K2_GetComponentToWorld` (`self.Arrow`))))
  (setmembers `/Game/VirtualVillageUE4/SubSystems/NPCSystemV5/Data/Structs/Station/S_Station_Info` :`StructRef` (`self.StationOptions`) :`Transform` (`KismetMathLibrary.MakeTransform` _returnvalue_location _returnvalue_rotation)))

(event `self.Tigger.OnComponentBeginOverlap`
  (params (OverlappedComponent :type "PrimitiveComponent Object Reference") (OtherActor :type "Actor Object Reference") (OtherComp :type "PrimitiveComponent Object Reference") (OtherBodyIndex :type Integer) (bFromSweep :type Boolean) (SweepResult :type "HitResult Structure (by ref)"))
  (bind _returnvalue (`self.GetComponentByClass` (`self.OverlappedActor`) "/Game/VirtualVillageUE4/SubSystems/NPCSystemV5/Blueprints/Characters/NPC/GenericAI/BPC_NPCController.BPC_NPCController_C"))
  (set `self.OverlappedActor` OtherActor)
  (`/Engine/EditorBlueprintResources/StandardMacros.IsValid` _returnvalue
    (:`Is Valid`
      (set `self.NPCController` _returnvalue)
      (`/Engine/EditorBlueprintResources/StandardMacros.DoOnce` false :!label _label
        (:`Completed`
          (message `/Game/VirtualVillageUE4/SubSystems/NPCSystemV5/Blueprints/Interfaces/BPI_NPC_Controller.ArrivedAtStation` (`self.NPCController`) self (`self.StationOptions`)))))))

(event `self.Tigger.OnComponentEndOverlap`
  (params (OverlappedComponent :type "PrimitiveComponent Object Reference") (OtherActor :type "Actor Object Reference") (OtherComp :type "PrimitiveComponent Object Reference") (OtherBodyIndex :type Integer))
  (bind _returnvalue (`self.GetComponentByClass` (`self.OverlappedActor`) "/Game/VirtualVillageUE4/SubSystems/NPCSystemV5/Blueprints/Characters/NPC/GenericAI/BPC_NPCController.BPC_NPCController_C"))
  (set `self.OverlappedActor` OtherActor)
  (`/Engine/EditorBlueprintResources/StandardMacros.IsValid` _returnvalue
    (:`Is Valid`
      (set `self.NPCController` _returnvalue)
      (goto _label :!via `Reset`))))

(event `/Game/VirtualVillageUE4/SubSystems/NPCSystemV5/Blueprints/Interfaces/BPI_Station.ShowHideProps`
  (params (`Show?` :type Boolean))
  (`SceneComponent.SetVisibility` (`self.Prop`) `Show?` false))

(fn `GetEntryPoint`
  (returns (`Entry Point` :type "Vector Structure"))
  (return (`SceneComponent.K2_GetComponentLocation` (`self.Arrow`))))

(fn `UserConstructionScript`
  (bind ((`AreaScale_2_D43DFAAD4A1163913C36C79236334099` _areascale) (`NavmeshvolumneScale_15_9EFE1926477CBA4E5418418430E0D492` _navmeshvolumnescale)) (break `/Game/VirtualVillageUE4/SubSystems/NPCSystemV5/Data/Structs/Station/S_Station_GeneralSettings` (`self.GeneralSettings`)))
  (bind ((`AreaVisible_5_DFB61A3E48F5A2D17458CB8B2D949D3A` _areavisible) (`AreaHidden_7_66EE875C4228C9C315FE388AF6A6DC67` _areahidden) (`PoseHidden_9_1F9DAC0343A77B5709FDCE99FDE2FC5F` _posehidden)) (break `/Game/VirtualVillageUE4/SubSystems/NPCSystemV5/Data/Structs/Station/S_Station_GeneralSettings` (`self.GeneralSettings`)))
  (bind ((`PropMesh_12_F59A7C6349DFA232849E2387659ACDDB` _propmesh) (`PoseMesh_18_7179FC204625D5BD8CEDEBA9D428075A` _posemesh)) (break `/Game/VirtualVillageUE4/SubSystems/NPCSystemV5/Data/Structs/Station/S_Station_GeneralSettings` (`self.GeneralSettings`)))
  (bind ((`PoseMesh_18_7179FC204625D5BD8CEDEBA9D428075A` _posemesh_2) (`PoseMaterial_21_1753FC7E422DD9761AEE9EBB005291F8` _posematerial)) (break `/Game/VirtualVillageUE4/SubSystems/NPCSystemV5/Data/Structs/Station/S_Station_GeneralSettings` (`self.GeneralSettings`)))
  ;[0 0 0] Area Scales
  (`SceneComponent.SetWorldScale3D` (`self.Area`) _areascale)
  (`SceneComponent.SetWorldScale3D` (`self.NavMeshBlocker`) _navmeshvolumnescale)
  ;[0 0 0] Visibilities
  (`SceneComponent.SetVisibility` (`self.Area`) _areavisible false)
  (`SceneComponent.SetHiddenInGame` (`self.Area`) _areahidden false)
  (`SceneComponent.SetHiddenInGame` (`self.PostSkeleton`) _posehidden false)
  ;[0 0 0] Set meshes
  (`StaticMeshComponent.SetStaticMesh` (`self.Prop`) _propmesh)
  (`SkinnedMeshComponent.SetSkinnedAssetAndUpdate` (`self.PostSkeleton`) _posemesh true)
  ;[0 0 0] Set materials
  (for (_ _array_index) (`SkeletalMesh.Materials` _posemesh_2)
    (`PrimitiveComponent.SetMaterial` (`self.PostSkeleton`) _array_index _posematerial)))